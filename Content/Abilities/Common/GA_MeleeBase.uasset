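; GA_MeleeBase is a common melee gameplay ability that plays an attack montage and applies effects when a hit event arrives.
; After committing, it runs PlayMontageAndWaitForEvent, listening for Event.Montage tags.
; Each received event applies the effect container keyed by its tag with the event data, then prints a debug string of tag, instigator and target.
; Montage completion, blend out, interruption or cancellation ends the ability, and OnEndAbility calls CallOnAbilityEnded.
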(event Ability|EventActivateAbility
  (bind _returnvalue (Ability|CommitAbility)) ; 提交能力，例如消耗法力值等操作
  (if _returnvalue
    (bind (_asynctaskproxy _eventtag _eventdata) (|PlayMontageandWaitforEvent "None" (Variables|Default|GetMontageToPlay) "(GameplayTags=((TagName=\"Event.Montage\")))" 1.0 "" true 1.0)
      (:OnComplete
        (Ability|EndAbility :!label _label) ; 没有接收到GameplayEvent就正常结束
      )
      (:OnBlendOut
        (goto _label))
      (:OnInterrupted
        (goto _label))
      (:OnCancelled
        (goto _label))
      (:EventReceived
        (Class|RPGGameplayAbility|ApplyEffectContainer _eventtag _eventdata -1) ; 收到GameEvent，简单的理解就是技能打到敌人了
        (Development|PrintString (Utilities|String|ToString(Text) (Utilities|Text|FormatText "ApplyEffectContainer:{TagName},InstigatorName:{Instigator}, TargetName:{TargetName}" (Utilities|Text|ToText(Name) (GameplayTags|GetTagName _eventtag)) (Utilities|Text|ToText(String) (Utilities|GetDisplayName (.Instigator (Utilities|Struct|BreakGameplayEventData _eventdata)))) (Utilities|Text|ToText(String) (Utilities|GetDisplayName (.Target (Utilities|Struct|BreakGameplayEventData _eventdata)))))))))))

(event Ability|EventOnEndAbility
  (params (bWasCancelled :type Boolean))
  (Default|CallOnAbilityEnded))