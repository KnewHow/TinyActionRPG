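; Base projectile Blueprint for abilities that applies a gameplay effect container to actors it overlaps.
; On overlap, it records each actor in HitActors so repeat overlaps are ignored, and skips applying effects to its instigator.
; Other actors are added as targets to the stored EffectContainerSpec, which is then applied as an external spec.
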(event EventBeginPlay)

(event Collision|EventActorBeginOverlap
  (params (OtherActor :type Actor%20Object%20Reference))
  (bind _hitactors (Variables|Default|GetHitActors))
  (if (not (Utilities|Array|ContainsItem _hitactors OtherActor))
    (Utilities|Array|Add _hitactors OtherActor)
    (if (!= OtherActor (Game|GetInstigator))
      (bind _returnvalue (Class|RPGBlueprintFunctionLibrary|AddTargetstoEffectContainerSpec (Variables|Default|GetEffectContainerSpec) 0 (Utilities|Array|MakeArray OtherActor))) ; 将目标添加到Spec
      (Class|RPGBlueprintFunctionLibrary|ApplyExternalEffectContainerSpec _returnvalue) ; 应用Spec
    )))

(event EventTick
  (params (DeltaSeconds :type Float%20%28single-precision%29)))

(fn ConstructionScript)