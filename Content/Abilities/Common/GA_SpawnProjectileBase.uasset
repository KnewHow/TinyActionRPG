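; Base gameplay ability that plays a montage and spawns a projectile when a montage event fires.
; After committing, it waits on Event.Montage events and builds an effect container spec from the received tag and data.
; If the spec has effects, it spawns ProjectileClass ahead of the avatar along its facing, handing over the spec and instigator so the projectile carries the effects.
; The ability ends when the montage completes, blends out, is interrupted or is cancelled.
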(event Ability|EventActivateAbility
  (bind _returnvalue (Ability|GetAvatarActorfromActorInfo))
  (bind _returnvalue_2 (Ability|CommitAbility))
  (if _returnvalue_2
    (bind (_asynctaskproxy _eventtag _eventdata) (|PlayMontageandWaitforEvent "None" (Variables|Default|GetMontageToPlay) "(GameplayTags=((TagName=\"Event.Montage\")))" 1.0 "None" true 1.0)
      (:OnComplete
        (Ability|EndAbility :!label _label))
      (:OnBlendOut
        (goto _label))
      (:OnInterrupted
        (goto _label))
      (:OnCancelled
        (goto _label))
      (:EventReceived
        (bind _returnvalue_3 (Class|RPGGameplayAbility|MakeEffectContainerSpec _eventtag _eventdata -1)) ; 把EffectContainerSpec交给外部的Actor
        (if (Class|RPGBlueprintFunctionLibrary|DoesEffectContainerSpecHaveEffects _returnvalue_3)
          (Game|SpawnActorfromClass (Variables|Default|GetProjectileClass) (Math|Transform|MakeTransform (+ (Transformation|GetActorLocation _returnvalue) (* (Math|Vector|Normalize (Transformation|GetActorForwardVector _returnvalue)) (Variables|Default|GetProjectilePawnLocationOffset))) (Transformation|GetActorRotation _returnvalue)) "AlwaysSpawn" 0 _returnvalue_3 (.AsPawn (Utilities|Casting|CastToPawn _returnvalue))))))))

(event Ability|EventOnEndAbility
  (params (bWasCancelled :type Boolean)))