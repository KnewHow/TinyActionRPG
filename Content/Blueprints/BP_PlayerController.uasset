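; Player controller that translates input into movement, camera and combat actions for BP_PlayerCharacter.
; On possess it tells the character to create its weapons, and movement follows control yaw unless BlockMovementInput is set.
; Mouse look feeds yaw and pitch directly, while gamepad look scales by base rate and delta time.
; Attack, roll and debug inputs forward to the character, with SkillAttack_01 switching to the second skill when moving forward.
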(event EventBeginPlay)

(event EventTick
  (params (DeltaSeconds :type Float%20%28single-precision%29)))

(event EventPossess
  (params (PossessedPawn :type Pawn%20Object%20Reference))
  (bind _asbp_player_character (Utilities|Casting|CastToBP_PlayerCharacter PossessedPawn))
  (Default|CreateAllWeapon _asbp_player_character))

(event Input|ActionEvents|InputActionNormalAttack
  (params (Key :type Key%20Structure :default "None"))
  (:Pressed
    (Default|DoNormalAttack (CallFunction|GetPlayerCharacterBP))))

(event Input|ActionEvents|InputActionSkillAttack_01
  (params (Key :type Key%20Structure :default "None"))
  (bind _result (CallFunction|GetPlayerCharacterBP))
  (:Pressed
    (if (> (Math|Vector|DotProduct (Transformation|GetActorForwardVector _result) (Transformation|GetVelocity _result)) 0.0)
      (Default|DoSkillAttack02 _result)
      (else
        (Default|DoSkillAttack01 _result)))))

(event Input|ActionEvents|InputActionComboAttaack
  (params (Key :type Key%20Structure :default "None"))
  (:Pressed
    (Default|JumpComboAttack (CallFunction|GetPlayerCharacterBP))))

(event Input|ActionEvents|InputActionRoll
  (params (Key :type Key%20Structure :default "None"))
  (:Pressed
    (Default|DoRoll (CallFunction|GetPlayerCharacterBP))))

(event Input|ActionEvents|InputActionDebugLaunchABall
  (params (Key :type Key%20Structure :default "None"))
  (:Pressed
    (Default|DebugLaunchABall (CallFunction|GetPlayerCharacterBP))))

(event Input|ActionEvents|InputActionSkillAttack_02
  (params (Key :type Key%20Structure :default "None"))
  (:Pressed
    (Default|DoSkillAttack02 (CallFunction|GetPlayerCharacterBP))))

(event Input|AxisEvents|InputAxisMoveRight
  (params (AxisValue :type Float%20%28single-precision%29))
  (bind _returnvalue (Game|Player|GetPlayerPawn 0))
  ;[1 1 1] 移动控制
  (Utilities|Casting|CastToBP_PlayerCharacter _returnvalue)
  (if (not (Variables|Default|GetBlockMovementInput))
    (Pawn|Input|AddMovementInput _returnvalue (Math|Vector|GetRightVector (Math|Rotator|MakeRotator 0.0 0.0 (.Yaw (Math|Rotator|BreakRotator (Pawn|GetControlRotation :!class /Script/Engine.Controller))))) AxisValue false)))

(event Input|AxisEvents|InputAxisTurn
  (params (AxisValue :type Float%20%28single-precision%29))
  ;[1 1 1] 使用鼠标旋转视角
  (Class|PlayerController|AddYawInput AxisValue))

(event Input|AxisEvents|InputAxisLookUp
  (params (AxisValue :type Float%20%28single-precision%29))
  ;[1 1 1] 使用鼠标旋转视角
  (Class|PlayerController|AddPitchInput AxisValue))

(event Input|AxisEvents|InputAxisTurnRate
  (params (AxisValue :type Float%20%28single-precision%29))
  ;[1 1 1] 使用手柄旋转，增加了一个基础的速率用来适配
  (Class|PlayerController|AddYawInput (* AxisValue (Variables|PlayerInputs|GetTurnRateBase) (Utilities|Time|GetWorldDeltaSeconds))))

(event Input|AxisEvents|InputAxisLookUpRate
  (params (AxisValue :type Float%20%28single-precision%29))
  ;[1 1 1] 使用手柄旋转，增加了一个基础的速率用来适配
  (Class|PlayerController|AddPitchInput (* AxisValue (Variables|PlayerInputs|GetLookupRateBase) (Utilities|Time|GetWorldDeltaSeconds))))

(event Input|AxisEvents|InputAxisMoveForward
  (params (AxisValue :type Float%20%28single-precision%29))
  (bind _returnvalue (Game|Player|GetPlayerPawn 0))
  ;[1 1 1] 移动控制
  (Utilities|Casting|CastToBP_PlayerCharacter _returnvalue)
  (if (not (Variables|Default|GetBlockMovementInput))
    (Pawn|Input|AddMovementInput _returnvalue (Math|Vector|GetForwardVector (Math|Rotator|MakeRotator 0.0 0.0 (.Yaw (Math|Rotator|BreakRotator (Pawn|GetControlRotation :!class /Script/Engine.Controller))))) AxisValue false)))

(fn ConstructionScript)