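; Base weapon actor whose capsule collision detects melee hits and notifies the instigator's Gameplay Abilities to apply damage.
; Animation notifies start and end each attack, setting the event tag and hit-pause settings and toggling query-only collision.
; An overlap with an actor of a different class than the instigator sends the Gameplay Event once, re-arming shortly after overlap ends.
; A limited, optional hit pause briefly slows global time dilation.
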(event Custom|Event%20BeginWeaponAttack
  (params (EventTag :type Gameplay%20Tag%20Structure) (AttackDelayTime :type Float%20%28single-precision%29) (AttackDelayCount :type Integer))
  ;[1 1 1] 此事件当攻击开始时通过AnimationNotify来调用，用设置此次攻击需要的标签、攻击后摇等信息
  (Variables|WeaponDefault|SetAttackEventTag EventTag)
  (Variables|WeaponDefault|SetAttackDelayTime AttackDelayTime)
  (Variables|WeaponDefault|SetAttackDelayCount AttackDelayCount)
  (Collision|SetCollisionEnabled (Variables|Default|GetCapsuleCollision) "QueryOnly") ; 开启碰撞
  (Variables|WeaponDefault|SetIsAttacking true))

(event Custom|Event%20EndedWeaponAttack
  ;[1 1 1] 当攻击结束时，修改状态和忽略碰撞，此事件依然通过Animation来调用
  (Variables|WeaponDefault|SetIsAttacking false)
  (Collision|SetCollisionEnabled (Variables|Default|GetCapsuleCollision) "NoCollision"))

(event Custom|HitPause
  ;[1 1 1] 攻击后摇
  (if (and (> (Variables|WeaponDefault|GetAttackDelayCount) 0) (Variables|WeaponDefault|GetEnableAttackDelay))
    (Math|Integer|DecrementInt (Variables|WeaponDefault|GetAttackDelayCount)
      (:%20%20
        (Utilities|FlowControl|Delay 0.1)
        (Utilities|Time|SetGlobalTimeDilation 0.1) ; 让游戏世界时间流速变慢，可以理解为慢镜头
        (Utilities|FlowControl|Delay 0.01)
        (Utilities|Time|SetGlobalTimeDilation 1.0) ; 恢复游戏时间正常时间流速
      ))))

(event EventBeginPlay
  ;[1 1 1] 当移动时忽略Actor
  (Collision|IgnoreActorwhenMoving (Variables|Default|GetCapsuleCollision) 0 false))

(event Collision|EventActorBeginOverlap
  (params (OtherActor :type Actor%20Object%20Reference))
  (bind _returnvalue (Game|GetInstigator))
  ;[1 1 1] 当Actor 碰到物体的时候，简单来说就是打到东西了
  (if (and (!= (Utilities|GetClass OtherActor) (Utilities|GetClass (Game|GetInstigator))) (Variables|WeaponDefault|GetIsAttacking)) ; 保证碰到的人不是自己
    (Utilities|FlowControl|DoOnce false
      (:Completed
        (Ability|SendGameplayEventtoActor _returnvalue (Variables|WeaponDefault|GetAttackEventTag) (Utilities|Struct|MakeGameplayEventData "" _returnvalue OtherActor)) ; 发送Gameplay Event 事件，用来通知GameAbility将伤害应用到目标上
        (CallFunction|HitPause)))))

(event Collision|EventActorEndOverlap
  (params (OtherActor :type Actor%20Object%20Reference))
  (bind _returnvalue (Game|GetInstigator))
  ;[1 1 1] 当结束碰撞的时候，重置攻击判断
  (Utilities|FlowControl|Delay 0.2)
  ;[1 1 1] 当Actor 碰到物体的时候，简单来说就是打到东西了
  (Utilities|FlowControl|DoOnce false) ; enters at Reset
)

(fn ConstructionScript)