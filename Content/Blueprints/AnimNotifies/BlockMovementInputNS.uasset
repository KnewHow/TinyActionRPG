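; Anim notify state that blocks the player's movement input during a marked window of an animation.
; Notify begin sets the BlockMovementInput flag on the player controller Blueprint, fetched using the mesh component as argument, and notify end clears it.
; Both events check that the mesh is valid, but only the end event also validates the controller.
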(fn ReceivedNotifyBegin
  (params (MeshComp :type Skeletal%20Mesh%20Component%20Object%20Reference) (Animation :type Anim%20Sequence%20Base%20Object%20Reference) (TotalDuration :type Float%20%28single-precision%29))
  (Utilities|IsValid MeshComp
    (:Is%20Valid
      (Variables|/Game/Blueprints/BP_PlayerController.BP_PlayerController_C|SetBlockMovementInput (CallFunction|GetPlayerControllerBP MeshComp) true)
      (return false))))

(fn ReceivedNotifyEnd
  (params (MeshComp :type Skeletal%20Mesh%20Component%20Object%20Reference) (Animation :type Anim%20Sequence%20Base%20Object%20Reference))
  (bind _result (CallFunction|GetPlayerControllerBP MeshComp))
  (if (and (Utilities|IsValid MeshComp) (Utilities|IsValid _result))
    (Variables|/Game/Blueprints/BP_PlayerController.BP_PlayerController_C|SetBlockMovementInput _result false)
    (return true)))