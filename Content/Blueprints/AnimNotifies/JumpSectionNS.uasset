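; JumpSectionNS is an animation notify state that marks the window during an animation in which the player character's combo period is open.
; On begin, it casts the mesh owner to BP_PlayerCharacter, sets EnableComboPeriod and stores itself as the character's JumpSectionNotify.
; On end, it clears EnableComboPeriod but leaves the stored notify reference in place.
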(fn ReceivedNotifyBegin
  (params (MeshComp :type Skeletal%20Mesh%20Component%20Object%20Reference) (Animation :type Anim%20Sequence%20Base%20Object%20Reference) (TotalDuration :type Float%20%28single-precision%29))
  (bind _asbp_player_character (Utilities|Casting|CastToBP_PlayerCharacter (Components|GetOwner MeshComp))
    (:then
      (Variables|/Game/Blueprints/BP_PlayerCharacter.BP_PlayerCharacter_C|SetEnableComboPeriod _asbp_player_character true)
      (Variables|/Game/Blueprints/BP_PlayerCharacter.BP_PlayerCharacter_C|SetJumpSectionNotify _asbp_player_character self)
      (return true))
    (:CastFailed
      (return true))))

(fn ReceivedNotifyEnd
  (params (MeshComp :type Skeletal%20Mesh%20Component%20Object%20Reference) (Animation :type Anim%20Sequence%20Base%20Object%20Reference))
  (bind _asbp_player_character (Utilities|Casting|CastToBP_PlayerCharacter (Components|GetOwner MeshComp))
    (:then
      (Variables|/Game/Blueprints/BP_PlayerCharacter.BP_PlayerCharacter_C|SetEnableComboPeriod _asbp_player_character false)
      (return true))
    (:CastFailed
      (return true))))