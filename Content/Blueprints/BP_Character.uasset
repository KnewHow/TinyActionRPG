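; BP_Character is a character Blueprint with shared combat helpers built on the Gameplay Ability System.
; DoNormalAttack activates the abilities bound to the current weapon slot, allowing remote activation.
; CanUseAnyAbility requires an unpaused game, health above zero and no active skill.
; Skill and melee checks query active abilities by gameplay tag, and the event graph and construction script are empty.
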(event EventBeginPlay)

(event Collision|EventActorBeginOverlap
  (params (OtherActor :type Actor%20Object%20Reference)))

(event EventTick
  (params (DeltaSeconds :type Float%20%28single-precision%29)))

(fn ConstructionScript)

(fn DoNormalAttack
  (Class|RPGCharacterBase|ActivateAbilitieswithItemSlot (Variables|Default|GetCurrentWeaponSlot) true))

(fn CanUseAnyAbility
  (return (Math|Boolean|ANDBoolean (not (Game|IsGamePaused)) (Health|IsAlive) (not (Attack|IsUsingSkill)))))

(fn IsAlive
  (return (> (Class|RPGCharacterBase|GetHealth) 0.0)))

(fn IsUsingSkill
  (bind _activeabilities (Class|RPGCharacterBase|GetActiveAbilitieswithTags (GameplayTags|MakeLiteralGameplayTagContainer "(GameplayTags=((TagName=\"Ability.Skill\")))")))
  (return (> (Utilities|Array|Length _activeabilities) 0)))

(fn IsUsingMelee
  (bind _activeabilities (Class|RPGCharacterBase|GetActiveAbilitieswithTags (GameplayTags|MakeLiteralGameplayTagContainer "(GameplayTags=((TagName=\"Ability.Melee\")))")))
  (return (> (Utilities|Array|Length _activeabilities) 0)))