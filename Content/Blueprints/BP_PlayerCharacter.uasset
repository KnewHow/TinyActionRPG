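; Player character Blueprint for an action RPG, providing normal attacks, melee combos, two slot-based skills and a roll.
; Normal attack advances the combo when melee is in use, otherwise activates the current weapon slot's ability.
; Combos chain by setting the montage's next section from JumpSectionNotify while the combo window is open, with a special jump to the final move.
; It also spawns slotted weapons on the hand socket and has a debug ball spawner.
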(event EventBeginPlay)

(event Collision|EventActorBeginOverlap
  (params (OtherActor :type Actor%20Object%20Reference)))

(event EventTick
  (params (DeltaSeconds :type Float%20%28single-precision%29)))

(fn ConstructionScript
  (|CallParentFunction))

(fn DoNormalAttack
  (if (CallFunction|CanUseAnyAbility)
    (if (CallFunction|IsUsingMelee)
      (Attack|DoComboAttack "Default")
      (else
        (Class|RPGCharacterBase|ActivateAbilitieswithItemSlot (Variables|Default|GetCurrentWeaponSlot) true) ; 单独的普通攻击
      ))))

(fn CreateAllWeapon
  (for _array_element (Class|RPGPlayerControllerBase|GetSlottedItems (CallFunction|GetPlayerControllerBP) "Weapon")
    (bind _asrpgweapon_item (Utilities|Casting|CastToRPGWeaponItem _array_element))
    (bind _returnvalue (Game|SpawnActorfromClass (Variables|/Script/ActionRPG.RPGWeaponItem|GetWeaponActor _asrpgweapon_item) (Math|Transform|MakeTransform "0, 0, 0") "Undefined" 0 0))
    (Transformation|AttachComponentToComponent _returnvalue (Variables|Character|GetMesh) "hand_rSocket" "KeepRelative" "KeepRelative" "KeepRelative" true)))

(fn DoComboAttack
  (params (JumpSection :type Name :default "Default"))
  (bind _jumpsectionnotify (Variables|Combo|GetJumpSectionNotify))
  (bind _mesh (Variables|Character|GetMesh))
  (bind _returnvalue (Components|SkeletalMesh|GetAnimInstance _mesh))
  (bind _returnvalue_2 (Animation|Montage|GetCurrentActiveMontage _returnvalue))
  (Utilities|IsValid _jumpsectionnotify
    (:Is%20Valid
      (if (Variables|Combo|GetEnableComboPeriod)
        (Class|AnimInstance|MontageSetNextSection _returnvalue (Animation|Montage|MontageGetCurrentSection _returnvalue _returnvalue_2) (select (Utilities|Name|Equal(Name) JumpSection "Default") (Variables|/Game/Blueprints/AnimNotifies/JumpSectionNS.JumpSectionNS_C|GetJumpSection _jumpsectionnotify) JumpSection) _returnvalue_2)))))

(fn JumpComboAttack
  ;[1 1 1] 跳转最后一招
  (if (Variables|Combo|GetEnableComboPeriod)
    (if (Utilities|Name|Equal(Name) (Variables|/Game/Blueprints/AnimNotifies/JumpSectionNS.JumpSectionNS_C|GetJumpSection (Variables|Combo|GetJumpSectionNotify)) "Comb-4")
      (Attack|DoComboAttack "Comb-5"))))

(fn DoRoll
  (if (not (Animation|Montage|MontageIsPlaying (Components|SkeletalMesh|GetAnimInstance (Variables|Character|GetMesh)) "/Game/Characters/Animations/AM_Roll.AM_Roll"))
    (Animation|PlayAnimMontage "/Game/Characters/Animations/AM_Roll.AM_Roll" 1.0 "None")))

(fn DoSkillAttack01
  (if (CallFunction|CanUseAnyAbility)
    (Class|RPGCharacterBase|ActivateAbilitieswithItemSlot (Utilities|Struct|MakeRPGItemSlot "Skill" 0) true)))

(fn DebugLaunchABall
  (bind _charactermovement (Variables|Character|GetCharacterMovement))
  (bind _returnvalue (Class|CharacterMovementComponent|GetCharacterOwner _charactermovement))
  (Game|SpawnActorfromClass "/Game/Blueprints/Test/Ball.Ball_C" (Math|Transform|MakeTransform (Transformation|GetActorLocation _returnvalue) (Transformation|GetActorRotation _returnvalue)) "AdjustIfPossibleButDontSpawnIfColliding" 0 0))

(fn DoSkillAttack02
  (if (CallFunction|CanUseAnyAbility)
    (Class|RPGCharacterBase|ActivateAbilitieswithItemSlot (Utilities|Struct|MakeRPGItemSlot "Skill" 1) true)))